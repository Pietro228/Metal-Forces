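; Matchmaking Blueprint that puts the player into an online multiplayer session, joining an existing one or hosting a new one.
; SearchGame looks for a single non-LAN session and joins the first result without checking that the list has entries.
; A failed search or join waits briefly, then creates a session and opens level A1 as a listen server.
; Each outcome is reported only through debug prints.
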(event `SearchGame`
  ;[1 1 1] Search for already existing Sessions
  (bind _results (`FindSessionsCallbackProxy.FindSessions` (`GameplayStatics.GetPlayerController` 0) 1)
    (:`OnSuccess`
      (set `self.SessionResults` _results)
      ;[1 1 1] Join already existing Session
      (`JoinSessionCallbackProxy.JoinSession` (`GameplayStatics.GetPlayerController` 0) (`|GetArrayItem` (`self.SessionResults`))
        (:`OnSuccess`
          (`KismetSystemLibrary.PrintString` "Session Joined"))
        (:`OnFailure`
          (`KismetSystemLibrary.PrintString` "CouldNotJoinSession")
          (`KismetSystemLibrary.Delay` 2.0 :!label _label)
          ;[1 1 1] If No Session is Found Create Session
          (`CreateSessionCallbackProxy.CreateSession` (`GameplayStatics.GetPlayerController` 0) 4
            (:`OnSuccess`
              (`KismetSystemLibrary.PrintString` "Session Created")
              (`GameplayStatics.OpenLevel` "A1" false "listen"))
            (:`OnFailure`
              (`KismetSystemLibrary.PrintString` "CouldNotCreateSession"))))))
    (:`OnFailure`
      (`KismetSystemLibrary.PrintString` "Session not found")
      (goto _label))))